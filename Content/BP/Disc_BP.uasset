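; Disc Blueprint with a function that picks a homing target for the disc.
; FindHomingTarget scans VRPawn actors tagged "Homing" and keeps the one nearest the disc.
; ClosestDistance is not reset within the function, so each comparison runs against its stored value.
; The function returns a SceneComponent from the chosen actor; the overlap event and construction script are empty.
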(event `self.ReceiveActorBeginOverlap`
  (params (OtherActor :type "Actor Object Reference")))

(fn `Find Homing Target`
  (returns (`Homing Target` :type "SceneComponent Object Reference"))
  (bind _outactors (`GameplayStatics.GetAllActorsOfClassWithTag` "/Game/VRTemplate/Blueprints/VRPawn.VRPawn_C" "Homing"))
  (for _array_element _outactors
    (bind _returnvalue (`KismetMathLibrary.VSize` (- (`self.K2_GetActorLocation` _array_element) (`self.K2_GetActorLocation`))))
    (if (< _returnvalue (`self.Closest Distance`))
      (set `self.Closest Distance` _returnvalue)
      (set `self.Homing Target` _array_element)))
  (return (`self.GetComponentByClass` (`self.Homing Target`) "/Script/Engine.SceneComponent")))

(fn `UserConstructionScript`)