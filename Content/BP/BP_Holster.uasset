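; BP_Holster is a holster actor that snaps an overlapping item tagged Interactable onto itself and holds one at a time.
; A HolsterMesh overlap passes through a DoOnce, then, if empty, attaches the item at the Holster socket and sets HasItem.
; It also marks the item's GrabComponent as holstered and gives it a holster reference.
; The CanHold? event re-arms the DoOnce after a short delay.
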(event `CanHold?`
  (bind _holstered (`self.Holstered`))
  (`KismetSystemLibrary.Delay` 1.0)
  (goto _label :!via `Reset`))

(event `self.HolsterMesh.OnComponentBeginOverlap`
  (params (OverlappedComponent :type "PrimitiveComponent Object Reference") (OtherActor :type "Actor Object Reference") (OtherComp :type "PrimitiveComponent Object Reference") (OtherBodyIndex :type Integer) (bFromSweep :type Boolean) (SweepResult :type "HitResult Structure (by ref)"))
  (bind _holstered (`self.Holstered`))
  (`/Engine/EditorBlueprintResources/StandardMacros.DoOnce` false :!label _label
    (:`Completed`
      (if (`self.ActorHasTag` OtherActor "Interactable")
        (if (not (`self.HasItem?`))
          (bind _output_get (set `self.Holstered` OtherActor))
          (bind _returnvalue (`self.GetComponentByClass` _output_get "/Game/VRTemplate/Blueprints/GrabComponent.GrabComponent_C"))
          (set `/Game/VRTemplate/Blueprints/GrabComponent.bISHolsted` true _returnvalue)
          (set `/Game/VRTemplate/Blueprints/GrabComponent.Holster` self _returnvalue)
          (`self.K2_SetActorLocation` _holstered (`SceneComponent.K2_GetComponentLocation` (`self.HolsterMesh`)) false true)
          (`self.K2_AttachToActor` _holstered self "Holster" "SnapToTarget" "SnapToTarget" "KeepRelative" true)
          (set `self.HasItem?` true))))))

(fn `UserConstructionScript`)